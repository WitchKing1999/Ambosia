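; PlainProjectile is a projectile that deals its attack points as damage to pawns it overlaps, then destroys itself.
; On overlap with another valid actor, it checks whether a pawn's controller derives from the Ambosia AI or player controller class.
; Damage is applied to that controller rather than the pawn, with the projectile's own controller as instigator.
; Any valid overlap destroys the projectile, even when no damage is dealt.
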(event `self.ReceiveActorBeginOverlap`
  (params (OtherActor :type "Actor Object Reference"))
  ;[1 1 1] When we hit something, we try to apply damage to the controller. In the end, we will destory ourself.
  (if (and (!= self OtherActor) (`KismetSystemLibrary.IsValid` OtherActor))
    (bind _aspawn (cast `Pawn` OtherActor)
      (:`then`
        (bind _returnvalue (`self.GetController` _aspawn))
        (bind _returnvalue_2 (`GameplayStatics.GetObjectClass` _returnvalue))
        (if (or (`KismetMathLibrary.ClassIsChildOf` _returnvalue_2 "/Game/Blueprints/Controllers/AmbosiaAIController.AmbosiaAIController_C") (`KismetMathLibrary.ClassIsChildOf` _returnvalue_2 "/Script/Ambosia.AmbosiaPlayerController"))
          (`GameplayStatics.ApplyDamage` _returnvalue (`self.AttackPoints`) (`self.GetController`) self "/Script/Ambosia.ProjectileDamageType")))
      (:`CastFailed`
        _))
    (`self.K2_DestroyActor`)))

(fn `UserConstructionScript`)