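; Behavior tree task that instantly turns the AI-controlled pawn to face the TargetPosition blackboard location.
; On execute, it takes the owning controller's pawn and computes yaw from the arctangent of the Y/X offset to the target, adding 180 degrees when the X offset is positive to fix the quadrant.
; Pitch and roll are zeroed, and the task then finishes successfully.
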(event `self.ReceiveExecute`
  (params (OwnerActor :type "Actor Object Reference"))
  (bind _ownedpawn (`self.OwnedPawn`))
  ;[1 1 1] Get our owned pawn and its location
  (bind _ascontroller (cast `Controller` OwnerActor))
  (bind _returnvalue (`Controller.K2_GetPawn` _ascontroller))
  (set `self.OwnedPawn` _returnvalue)
  (bind _returnvalue_2 (- (`Actor.K2_GetActorLocation` _returnvalue) (`BTFunctionLibrary.GetBlackboardValueAsVector` (`self.Target Position`))))
  ;[1 1 1] the calculated angle needs to be converted to an Unreal rotation value
  (if (> (.x _returnvalue_2) 0.0)
    (bind _returnvalue_3 (`KismetMathLibrary.DegAtan` (/ (.y _returnvalue_2) (.x _returnvalue_2))))
    (`Actor.SetActorRotation` _ownedpawn (`KismetMathLibrary.MakeRotator` 0.0 0.0 (+ _returnvalue_3 180.0)))
    (else
      (`Actor.SetActorRotation` _ownedpawn (`KismetMathLibrary.MakeRotator` 0.0 0.0 _returnvalue_3))))
  (`self.FinishExecute` true))