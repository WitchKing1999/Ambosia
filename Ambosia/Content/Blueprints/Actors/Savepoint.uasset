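; Savepoint actor that saves the player's progress to the "Ambosia" slot when the player pawn overlaps it.
; It creates a fresh AmbosiaSavegame, copying health, mana and attack stats from the controller's GameplaySystemComponent, and experience, skill points and level from AmbosiaPlayerController.
; The stored respawn transform sits slightly in front of the savepoint, facing its rotation.
; A printed message reports whether saving succeeded.
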(event `self.ReceiveBeginPlay`)

(event `self.ReceiveActorBeginOverlap`
  (params (OtherActor :type "Actor Object Reference")))

(event `self.ReceiveTick`
  (params (DeltaSeconds :type "Float (single-precision)")))

(event `self.ReceiveActorBeginOverlap`
  (params (OtherActor :type "Actor Object Reference"))
  (bind _returnvalue (`GameplayStatics.GetPlayerController` 0))
  (bind _returnvalue_2 (`self.K2_GetActorRotation`))
  (bind _item (`KismetArrayLibrary.Array_Get` (`self.K2_GetComponentsByClass` _returnvalue "/Script/Ambosia.GameplaySystemComponent")))
  (if (== OtherActor (`GameplayStatics.GetPlayerPawn` 0))
    (bind _asambosia_player_controller (cast `/Game/Blueprints/Controllers/AmbosiaPlayerController` _returnvalue))
    (if (!= _returnvalue null)
      (if (!= _item null)
        (bind _returnvalue_3 (`GameplayStatics.CreateSaveGameObject` "/Game/Blueprints/AmbosiaSavegame.AmbosiaSavegame_C"))
        (bind _asambosia_savegame (cast `/Game/Blueprints/AmbosiaSavegame` _returnvalue_3))
        (set `/Game/Blueprints/AmbosiaSavegame.HealthPoints` (`GameplaySystemComponent.HealthPoints` _item) _asambosia_savegame)
        (set `/Game/Blueprints/AmbosiaSavegame.HealthPointsLimit` (`GameplaySystemComponent.HealthPointsLimit` _item) _asambosia_savegame)
        (set `/Game/Blueprints/AmbosiaSavegame.Mana` (`GameplaySystemComponent.Mana` _item) _asambosia_savegame)
        (set `/Game/Blueprints/AmbosiaSavegame.ManaLimit` (`GameplaySystemComponent.ManaLimit` _item) _asambosia_savegame)
        (set `/Game/Blueprints/AmbosiaSavegame.ManaRegeneration` (`GameplaySystemComponent.ManaRegenerationPerSec` _item) _asambosia_savegame)
        (set `/Game/Blueprints/AmbosiaSavegame.AttackPoints` (`GameplaySystemComponent.AttackPoints` _item) _asambosia_savegame)
        (set `/Game/Blueprints/AmbosiaSavegame.MagicalAttackPoints` (`GameplaySystemComponent.MagicalAttackPoints` _item) _asambosia_savegame)
        (set `/Game/Blueprints/AmbosiaSavegame.ExperiencePoints` (`/Game/Blueprints/Controllers/AmbosiaPlayerController.ExperiencePoints` _asambosia_player_controller) _asambosia_savegame)
        (set `/Game/Blueprints/AmbosiaSavegame.SkillPoints` (`/Game/Blueprints/Controllers/AmbosiaPlayerController.SkillPoints` _asambosia_player_controller) _asambosia_savegame)
        (set `/Game/Blueprints/AmbosiaSavegame.SkillLevel` (`/Game/Blueprints/Controllers/AmbosiaPlayerController.CurrentLevel` _asambosia_player_controller) _asambosia_savegame)
        (set `/Game/Blueprints/AmbosiaSavegame.Spawnpoint` (`KismetMathLibrary.MakeTransform` (+ (`self.K2_GetActorLocation`) (`KismetMathLibrary.GreaterGreater_VectorRotator` (96.0 0.0 0.0) _returnvalue_2)) _returnvalue_2) _asambosia_savegame)
        (bind _returnvalue_4 (`GameplayStatics.SaveGameToSlot` _asambosia_savegame "Ambosia"))
        (if _returnvalue_4
          (`KismetSystemLibrary.PrintString` "Game Saved!")
          (else
            (`KismetSystemLibrary.PrintString` "Saving failed!")))))))

(fn `UserConstructionScript`)