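; Spawner actor that keeps one instance of a configurable actor class in the world, replacing it when it is gone.
; Tick checks for an empty current actor and uses a running flag to allow only one pending delay.
; After the delay, it spawns the actor at its own transform and binds its EndPlay event to clear the reference, which restarts the cycle.
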(event `self.ReceiveTick`
  (params (DeltaSeconds :type "Float (single-precision)"))
  (if (and (== (`self.CurrentActor`) null) (not (`self.SpawnDelayRunning`)))
    (set `self.SpawnDelayRunning` true)
    (`KismetSystemLibrary.Delay` (`self.SpawnDelay`))
    ;[1 1 1] Spawning the actor
    (bind _returnvalue (`|SpawnActorFromClass` (`self.SpawnActorType`) (`self.GetTransform`) "Undefined" "OverrideRootScale"))
    (bind _output_get (set `self.CurrentActor` _returnvalue))
    (add `self.OnEndPlay` _output_get (delegate `OnEndPlay(Current Actor)`))
    (set `self.SpawnDelayRunning` false)))

(event `OnEndPlay(Current Actor)` :!signature `self.OnEndPlay`
  (params (EndPlayReason :type "EEndPlayReason Enum"))
  ;[1 1 1] when the actor dies, reset our current actor
  (set `self.CurrentActor` null))

(fn `UserConstructionScript`)