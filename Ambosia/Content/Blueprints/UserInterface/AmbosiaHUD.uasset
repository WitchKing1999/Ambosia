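; AmbosiaHUD manages the player's on-screen UI: life/XP bars, hero menu, interact icon, quit-to-main-menu prompt and save indicator.
; On BeginPlay it creates the bars and hero menu widgets, starting with the menu collapsed and bars visible.
; Events toggle widget visibility and open flags, with the inventory also switching between UI-only and game-only input.
; It binds to AmbosiaPlayerController's OnGameSaved event to show an indicator after successful saves.
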(event `self.ReceiveBeginPlay`
  ;[1 1 1] Create HUD
  (bind _returnvalue (`|CreateWidget` "/Game/Blueprints/UserInterface/IngameHUD/AmbosiaHUD_LifeXP_Bar.AmbosiaHUD_LifeXP_Bar_C"))
  (bind _output_get (set `self.BarsHUD` _returnvalue))
  (`UserWidget.AddToViewport` _output_get 0)
  ;[1 1 1] Create Hero Menu
  (bind _returnvalue_2 (`|CreateWidget` "/Game/Blueprints/UserInterface/Interfaces/HeroMenuWidget.HeroMenuWidget_C"))
  (bind _output_get_2 (set `self.InventoryHUD` _returnvalue_2))
  (`UserWidget.AddToViewport` _output_get_2 0)
  (`self.CloseInventory`)
  (`self.ShowHUD`)
  ;[1 1 1] When the game is saved, we will create a "saved" indicator
  (bind _asambosia_player_controller (cast `AmbosiaPlayerController` (`GameplayStatics.GetPlayerController` 0)))
  (bind _output_get_3 (set `self.PlayerControllerReference` _asambosia_player_controller))
  (add `AmbosiaPlayerController.OnGameSaved` _output_get_3 (`|CreateDelegate` :!event `OnGameSaved`)))

(event `self.OpenInventory`
  (bind _inventoryhud (`self.InventoryHUD`))
  (`Widget.SetVisibility` _inventoryhud "Visible")
  (set `self.bInventoryOpen` true)
  (`WidgetBlueprintLibrary.SetInputMode_UIOnlyEx` (`GameplayStatics.GetPlayerController` 0) _inventoryhud true))

(event `self.CloseInventory`
  (`Widget.SetVisibility` (`self.InventoryHUD`) "Collapsed")
  (set `self.bInventoryOpen` false)
  (`WidgetBlueprintLibrary.SetInputMode_GameOnly` (`GameplayStatics.GetPlayerController` 0)))

(event `self.ShowHUD`
  (`Widget.SetVisibility` (`self.BarsHUD`) "Visible")
  (set `self.bHUDOpen` true))

(event `self.HideHUD`
  (`Widget.SetVisibility` (`self.BarsHUD`) "Collapsed")
  (set `self.bHUDOpen` false))

(event `self.OpenReturnToMainMenuWidget`
  (bind _returnvalue (`|CreateWidget` "/Game/Blueprints/UserInterface/Interfaces/QuitToMainMenuWidget.QuitToMainMenuWidget_C"))
  (`UserWidget.AddToViewport` _returnvalue 0))

(event `self.ShowInteractIcon`
  (bind _returnvalue (`|CreateWidget` "/Game/Blueprints/UserInterface/IngameHUD/InteractIcon.InteractIcon_C"))
  (bind _output_get (set `self.InteractIcon` _returnvalue))
  (`UserWidget.AddToViewport` _output_get 0))

(event `self.HideInteractIcon`
  (`Widget.RemoveFromParent` (`self.InteractIcon`))
  (set `self.InteractIcon` null))

(fn `OnGameSaved`
  (params (Successfull :type Boolean))
  (if Successfull
    (bind _returnvalue (`|CreateWidget` "/Game/Blueprints/UserInterface/IngameHUD/AmbosiaHUD_OnSavedIndicator.AmbosiaHUD_OnSavedIndicator_C"))
    (`UserWidget.AddToViewport` _returnvalue 0)))

(fn `UserConstructionScript`)