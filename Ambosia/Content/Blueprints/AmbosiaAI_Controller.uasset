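; AI controller for the Ambosia character that handles its sword damage and health.
; A sword damage event sends AttackPoints through the IDamagable interface to any implementing actor except its own pawn, first retracting the pawn's sword.
; The controller holds the health, subtracting incoming deltas, capping at the limit and destroying the controlled pawn at zero or below.
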(event `/Game/Blueprints/iInterestedController.doSwordDamage`
  (params (OtherActor :type "Actor Object Reference"))
  ;[1 1 1] only do damage if the other actor is damagable and it's not the controlled pawn
  (if (and (!= (`self.K2_GetPawn`) OtherActor) (`KismetSystemLibrary.DoesImplementInterface` OtherActor "/Game/Blueprints/iDamagable.iDamagable_C"))
    ;[1 1 1] retract the sword of the ambosia character
    (bind _asambosia_character (cast `/Game/Blueprints/AmbosiaCharacter` (`self.K2_GetPawn`))
      (:`then`
        (`/Game/Blueprints/AmbosiaCharacter.MoveSword` _asambosia_character false))
      (:`CastFailed`
        _))
    ;[1 1 1] do the damage
    (message `/Game/Blueprints/iDamagable.AffectHealthPoints` OtherActor (`self.AttackPoints`))))

(event `/Game/Blueprints/iInterestedController.AffectHealthPoints`
  (params (Delta :type "Float (single-precision)"))
  (bind _healthpointslimit (`self.HealthPointsLimit`))
  ;[1 1 1] affect the health points
  (bind _output_get (set `self.HealthPoints` (- (`self.HealthPoints`) Delta)))
  ;[1 1 1] if the health points are greater than the limit, set them to the limit
  (if (> _output_get _healthpointslimit)
    (bind _output_get_2 (set `self.HealthPoints` _healthpointslimit))
    (else
      ;[1 1 1] if the health points are equal or below 0, die!
      (if (<= _output_get_2 0.0)
        (`self.Die`)))))

(fn `Die`
  (`self.K2_DestroyActor` (`self.K2_GetPawn`)))

(fn `UserConstructionScript`)