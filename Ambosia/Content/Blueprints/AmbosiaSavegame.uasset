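; AmbosiaSavegame is a save game Blueprint that holds the player's inventory and equipped item state.
; Its ClearItems function empties the Items and ItemStacks arrays.
; It also resets the equipped slot indices for weapon, armor, potion, arrow bundle, two rings and amulet to -1, marking them as unset.
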(fn `ClearItems`
  (set `self.Items` (`|MakeArray`))
  (set `self.ItemStacks` (`|MakeArray`))
  (set `self.WeaponIndex` -1)
  (set `self.ArmorIndex` -1)
  (set `self.PotionIndex` -1)
  (set `self.ArrowBundleIndex` -1)
  (set `self.FirstRingIndex` -1)
  (set `self.SecondRingIndex` -1)
  (set `self.AmuletIndex` -1))