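; Player controller for Ambosia that handles movement, yaw look, weapon and potion use, damage and character progression.
; On BeginPlay it equips default items through GameplaySystem, then restores stats and progression from the "Ambosia" save slot.
; Loot adds experience; item creation runs only on level-up, alongside skill point awards.
; SpendSkillPoints raises a chosen stat; the Inventory key currently buys health limit, and MainMenu quits as a placeholder.
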(event `self.ReceiveBeginPlay`
  (bind _gameplaysystem (`self.GameplaySystem`))
  ;[1 1 1] damage handling
  (add `self.OnTakeAnyDamage` (delegate `OnTakeAnyDamage_Event_0`))
  ;[1 1 1] activating our items
  (`GameplaySystemComponent.SetArmor` (`self.GameplaySystem`) (`self.PlainArmor`))
  (`GameplaySystemComponent.SetPotion` (`self.GameplaySystem`) (`self.50_HP_Potion`))
  (`GameplaySystemComponent.SetArrowBundle` (`self.GameplaySystem`) (`self.PlainArrowBundle`))
  (`GameplaySystemComponent.SetWeapon` (`self.GameplaySystem`) (`self.SuperBow`))
  (`GameplaySystemComponent.SetFirstRing` (`self.GameplaySystem`) (`self.PlainRing`))
  ;[1 1 1] Loading the last save
  (bind _returnvalue (`GameplayStatics.LoadGameFromSlot` "Ambosia"))
  (bind _asambosia_savegame (cast `/Game/Blueprints/AmbosiaSavegame` _returnvalue))
  (`GameplaySystemComponent.SetHealthPointsLimit` _gameplaysystem (`/Game/Blueprints/AmbosiaSavegame.HealthPointsLimit` _asambosia_savegame))
  (`GameplaySystemComponent.SetHealthPoints` _gameplaysystem (`/Game/Blueprints/AmbosiaSavegame.HealthPoints` _asambosia_savegame))
  (`GameplaySystemComponent.SetManaLimit` _gameplaysystem (`/Game/Blueprints/AmbosiaSavegame.ManaLimit` _asambosia_savegame))
  (`GameplaySystemComponent.SetMana` _gameplaysystem (`/Game/Blueprints/AmbosiaSavegame.Mana` _asambosia_savegame))
  (`GameplaySystemComponent.SetManaRegenerationPerSec` _gameplaysystem (`/Game/Blueprints/AmbosiaSavegame.ManaRegeneration` _asambosia_savegame))
  (`GameplaySystemComponent.SetAttackPoints` _gameplaysystem (`/Game/Blueprints/AmbosiaSavegame.AttackPoints` _asambosia_savegame))
  (`GameplaySystemComponent.SetMagicalAttackPoints` _gameplaysystem (`/Game/Blueprints/AmbosiaSavegame.MagicalAttackPoints` _asambosia_savegame))
  (set `self.ExperiencePoints` (`/Game/Blueprints/AmbosiaSavegame.ExperiencePoints` _asambosia_savegame))
  (set `self.SkillPoints` (`/Game/Blueprints/AmbosiaSavegame.SkillPoints` _asambosia_savegame))
  (set `self.CurrentLevel` (`/Game/Blueprints/AmbosiaSavegame.SkillLevel` _asambosia_savegame))
  (`KismetSystemLibrary.PrintString` "Save loaded!"))

(event `OnTakeAnyDamage_Event_0` :!signature `self.OnTakeAnyDamage`
  (params (Damage :type "Float (double-precision)") (DamageType :type "DamageType Object Reference") (InstigatedBy :type "Controller Object Reference") (DamageCauser :type "Actor Object Reference"))
  ;[1 1 1] damage handling
  (`GameplaySystemComponent.TakeDamage` (`self.GameplaySystem`) Damage DamageType InstigatedBy DamageCauser))

(event `InputAxis|MoveForward`
  (params (AxisValue :type "Float (single-precision)"))
  ;[1 1 1] movement controlls
  (`Pawn.AddMovementInput` (`self.K2_GetPawn`) (`KismetMathLibrary.GetForwardVector` (`self.GetControlRotation`)) AxisValue false))

(event `InputAxis|LookRight`
  (params (AxisValue :type "Float (single-precision)"))
  ;[1 1 1] rotation control
  (`self.AddYawInput` (* AxisValue (`self.LookRate`))))

(event `InputAxis|MoveRight`
  (params (AxisValue :type "Float (single-precision)"))
  ;[1 1 1] movement controlls
  (`Pawn.AddMovementInput` (`self.K2_GetPawn`) (`KismetMathLibrary.GetRightVector` (`self.GetControlRotation`)) AxisValue false))

(event `InputAction|Attack`
  (params (Key :type "Key Structure" :default "AnyKey"))
  (bind _weapon (`GameplaySystemComponent.Weapon` (`self.GameplaySystem`)))
  ;[1 1 1] attack controll
  (:`Pressed`
    (if (!= _weapon null)
      (`ItemComponent.Action` _weapon))))

(event `InputAction|Potion`
  (params (Key :type "Key Structure" :default "AnyKey"))
  (bind _potion (`GameplaySystemComponent.Potion` (`self.GameplaySystem`)))
  ;[1 1 1] potion controll
  (:`Pressed`
    (if (!= _potion null)
      (`ItemComponent.Action` _potion))))

(event `InputAction|MainMenu`
  (params (Key :type "Key Structure" :default "AnyKey"))
  ;[1 1 1] This will be replaced when main menu is ready
  (:`Pressed`
    (`KismetSystemLibrary.QuitGame` null "Quit")))

(event `/Game/Blueprints/Interfaces/LootCollector.Receive Loot`
  (params (ItemClasses :type "Array of ItemComponent Class Reference (by ref)") (ItemStacks :type "Array of Integer (by ref)") (Experience :type "Float (single-precision)"))
  (bind _returnvalue (+ (`self.CurrentLevel`) 1))
  ;[1 1 1] Experience handling
  (bind _output_get (set `self.ExperiencePoints` (+ (`self.ExperiencePoints`) Experience)))
  (if (< _returnvalue (`KismetArrayLibrary.Array_Length` (`self.XPLevels`)))
    (if (>= _output_get (`KismetArrayLibrary.Array_Get` (`self.XPLevels`) _returnvalue))
      (bind _output_get_2 (set `self.CurrentLevel` (+ (`self.CurrentLevel`) 1)))
      (set `self.SkillPoints` (+ (`KismetArrayLibrary.Array_Get` (`self.SkillPointsList`) _output_get_2) (`self.SkillPoints`)))
      ;[1 1 1] Loot handling
      (for (_array_element _array_index) ItemClasses
        (bind _returnvalue_2 (`GameplaySystemComponent.CreateAndAddItem` (`self.GameplaySystem`) _array_element))
        (`ItemComponent.SetStackSize` _returnvalue_2 (`KismetArrayLibrary.Array_Get` ItemStacks _array_index))))))

(event `InputAction|Inventory`
  (params (Key :type "Key Structure" :default "AnyKey"))
  (:`Pressed`
    (`self.SpendSkillPoints` 5.0 "NewEnumerator0")))

(fn `SpendSkillPoints`
  (params (Amount :type "Float (double-precision)") (Value :type "/Game/Blueprints/Enums/SkillableValue Enum"))
  (bind _gameplaysystem (`self.GameplaySystem`))
  (if (<= Amount (`self.SkillPoints`))
    (switch `/Game/Blueprints/Enums/SkillableValue` Value
      (:`NewEnumerator0`
        (`GameplaySystemComponent.AffectHealthPointsLimit` _gameplaysystem Amount))
      (:`NewEnumerator1`
        (`GameplaySystemComponent.AffectManaLimit` _gameplaysystem Amount))
      (:`NewEnumerator4`
        (`GameplaySystemComponent.AffectManaRegeneration` _gameplaysystem Amount))
      (:`NewEnumerator2`
        (`GameplaySystemComponent.AffectAttackPoints` _gameplaysystem Amount))
      (:`NewEnumerator3`
        (`GameplaySystemComponent.AffectMagicalAttackPoints` _gameplaysystem Amount)))
    (set `self.SkillPoints` (- (`self.SkillPoints`) Amount))))

(fn `UserConstructionScript`)