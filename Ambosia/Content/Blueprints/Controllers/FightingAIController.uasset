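; AI controller for combat pawns that handles incoming damage and rewards the player on death.
; Damage is recorded by instigator and forwarded to GameplaySystem, whose damage event is bound to spawn a damage indicator widget at the pawn's location.
; When destroyed after a last hit from an AmbosiaPlayerController, it rolls each child ItemComponent's drop chance and sends that player the loot and experience.
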(event `self.ReceiveBeginPlay`
  ;[1 1 1] Damage Handling
  (add `self.OnTakeAnyDamage` (delegate `OnTakeDamage`))
  ;[1 1 1] Create a damage indicator when we got hit
  (add `GameplaySystemComponent.OnDamageTook` (`self.GameplaySystem`) (`|CreateDelegate` :!event `CreateDamageIndicator`)))

(event `OnTakeDamage` :!signature `self.OnTakeAnyDamage`
  (params (Damage :type "Float (double-precision)") (DamageType :type "DamageType Object Reference") (InstigatedBy :type "Controller Object Reference") (DamageCauser :type "Actor Object Reference"))
  ;[1 1 1] Damage Handling
  (set `self.LastDamageInstigator` InstigatedBy)
  (`GameplaySystemComponent.TakeDamage` (`self.GameplaySystem`) Damage DamageType InstigatedBy DamageCauser))

(event `self.ReceiveEndPlay`
  (params (EndPlayReason :type "EEndPlayReason Enum" :default "Destroyed"))
  ;[1 1 1] Only drop loot when we were destroied and the player has killed us
  (switch `EEndPlayReason` EndPlayReason
    (:`Destroyed`
      (bind _asambosia_player_controller (cast `AmbosiaPlayerController` (`self.LastDamageInstigator`)))
      (for _array_element (`SceneComponent.GetChildrenComponents` (`self.GameplaySystem`) false)
        ;[1 1 1] Generate a random number and if the drop chance of the item is equal or below it, we will drop this item
        (bind _asitem_component (cast `ItemComponent` _array_element))
        (if (<= (`KismetMathLibrary.RandomFloatInRange` 0.0 1.0) (`ItemComponent.DropChance` _asitem_component))
          (`KismetArrayLibrary.Array_Add` (`self.LootItemClasses`) (`GameplayStatics.GetObjectClass` _asitem_component))
          (`KismetArrayLibrary.Array_Add` (`self.LootItemStacks`) (`ItemComponent.StackSize` _asitem_component))))
      (`AmbosiaPlayerController.ReceiveLoot` _asambosia_player_controller (`self.LootItemClasses`) (`self.LootItemStacks`) (`self.ExperienceGain`)))))

(fn `CreateDamageIndicator`
  (params (RawDamageAmount :type "Float (double-precision)") (DamageAmount :type "Float (double-precision)") (DamageType :type "DamageType Object Reference") (DamagingActor :type "Actor Object Reference"))
  (bind _returnvalue (`|CreateWidget` "/Game/Blueprints/UserInterface/IngameHUD/DamageIndicatorWidget.DamageIndicatorWidget_C"))
  (set `/Game/Blueprints/UserInterface/IngameHUD/DamageIndicatorWidget.DamageAmount` DamageAmount _returnvalue)
  (set `/Game/Blueprints/UserInterface/IngameHUD/DamageIndicatorWidget.ActorLocation` (`self.K2_GetActorLocation` (`self.K2_GetPawn`)) _returnvalue)
  (`UserWidget.AddToViewport` _returnvalue 0))

(fn `UserConstructionScript`)