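; ShooterAI is an AI controller for a bow-wielding shooter that targets the player.
; On BeginPlay it sets up the ShooterBB blackboard, equips a plain bow and arrow bundle through GameplaySystem, and runs the ShooterBT behavior tree.
; Every tick it writes the first player pawn's location into the blackboard's target position key, with no perception or line-of-sight check.
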(event EventTick
  (params (DeltaSeconds :type Float%20%28single-precision%29))
  (CallFunction|UpdateBlackboard))

(event EventBeginPlay
  (|CallParentFunction)
  (bind _blackboardcomponent (Class|AIController|UseBlackboard "/Game/AIs/ShooterBB.ShooterBB"))
  (Variables|Default|SetUsedBlackboard _blackboardcomponent)
  (Class|GameplaySystemComponent|SetWeapon (Variables|Default|GetGameplaySystem) (Variables|Default|GetPlainBow))
  (Class|GameplaySystemComponent|SetArrowBundle (Variables|Default|GetGameplaySystem) (Variables|Default|GetPlainArrowBundle))
  (AI|RunBehaviorTree "/Game/AIs/ShooterBT.ShooterBT"))

(fn ConstructionScript)

(fn UpdateBlackboard
  (AI|Components|Blackboard|SetValueasVector (Variables|Default|GetUsedBlackboard) (LocalVariables|GetTargetPositionKey) (Transformation|GetActorLocation (Game|Player|GetPlayerPawn 0))))