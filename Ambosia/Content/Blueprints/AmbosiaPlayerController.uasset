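; AmbosiaPlayerController is a player controller that handles movement, turning and item use for the player.
; Axis inputs move the controlled pawn along the control rotation's forward and right vectors and apply yaw scaled by LookRate.
; Attack and Potion inputs trigger the equipped Inventory weapon or potion, with starting armor, bow and potion set in the construction script.
; Destruction of the controller quits the game.
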(event `InputAxis|MoveForward`
  (params (AxisValue :type "Float (single-precision)"))
  (`Pawn.AddMovementInput` (`self.K2_GetPawn`) (`KismetMathLibrary.GetForwardVector` (`self.GetControlRotation`)) AxisValue false))

(event `InputAxis|MoveRight`
  (params (AxisValue :type "Float (single-precision)"))
  (`Pawn.AddMovementInput` (`self.K2_GetPawn`) (`KismetMathLibrary.GetRightVector` (`self.GetControlRotation`)) AxisValue false))

(event `InputAxis|LookRight`
  (params (AxisValue :type "Float (single-precision)"))
  (`self.AddYawInput` (* AxisValue (`self.LookRate`))))

(event `InputAction|Attack`
  (params (Key :type "Key Structure" :default "AnyKey"))
  (bind _weapon (`InventoryComponent.Weapon` (`self.Inventory`)))
  (:`Pressed`
    (if (!= _weapon null)
      (`ItemComponent.Action` _weapon))))

(event `self.ReceiveDestroyed`
  (`KismetSystemLibrary.QuitGame` null "Quit"))

(event `InputAction|Potion`
  (params (Key :type "Key Structure" :default "AnyKey"))
  (bind _potion (`InventoryComponent.Potion` (`self.Inventory`)))
  (:`Pressed`
    (if (!= _potion null)
      (`ItemComponent.Action` _potion))))

(fn `UserConstructionScript`
  (`InventoryComponent.SetArmor` (`self.Inventory`) (`self.PlainArmor`))
  (`InventoryComponent.SetWeapon` (`self.Inventory`) (`self.PlainBow`))
  (`InventoryComponent.SetPotion` (`self.Inventory`) (`self.50_HP_Potion`)))