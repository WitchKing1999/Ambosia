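; Behavior tree task that snaps the AI-controlled pawn's yaw to face the TargetPosition blackboard vector.
; It takes the arctangent of the Y/X offset between pawn and target, adding 180 degrees when needed to resolve the quadrant.
; The rotation is set instantly with pitch and roll zeroed, then the task finishes successfully.
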(event `self.ReceiveExecute`
  (params (OwnerActor :type "Actor Object Reference"))
  (bind _ownedpawn (`self.OwnedPawn`))
  (bind _ascontroller (cast `Controller` OwnerActor))
  (bind _returnvalue (`Controller.K2_GetPawn` _ascontroller))
  (set `self.OwnedPawn` _returnvalue)
  (bind _returnvalue_2 (- (`Actor.K2_GetActorLocation` _returnvalue) (`BTFunctionLibrary.GetBlackboardValueAsVector` (`self.Target Position`))))
  (set `self.deltaVector` _returnvalue_2)
  (set `self.alpha` (`KismetMathLibrary.DegAtan` (/ (.y _returnvalue_2) (.x _returnvalue_2))))
  (if (> (.x (`self.deltaVector`)) 0.0)
    (`Actor.SetActorRotation` _ownedpawn (`KismetMathLibrary.MakeRotator` 0.0 0.0 (+ (`self.alpha`) 180.0)))
    (else
      (`Actor.SetActorRotation` _ownedpawn (`KismetMathLibrary.MakeRotator` 0.0 0.0 (`self.alpha`)))))
  (`self.FinishExecute` true))